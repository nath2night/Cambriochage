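; Pastry collectible that spins in place and is picked up when a BP_ThirdPersonCharacter overlaps it.
; The construction script picks mesh and scale from TypeCollectible, while BeginPlay loops a rotation timeline and sets Score from a separate Gateau selector.
; Pickup increments the character's Butin by one, ignoring Score, then destroys the actor and prints the count.
; At the carry limit it only prints "full".
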(event `self.ReceiveBeginPlay`
  (`|ExecutionSequence`
    (:`then_0`
      (bind (_direction _rotation) (`Timeline|Rotation_Collectible` :!label _label)
        (:`Update`
          (`SceneComponent.K2_SetRelativeRotation` (`self.Cube`) (`KismetMathLibrary.MakeRotator` 0.0 0.0 _rotation) false false))
        (:`Finished`
          (`self.replay`))))
    (:`then_1`
      (set `self.Score` (select `/Game/Blueprints/Viennoiseries/Enum_ScoreGateaux` "NewEnumerator0" :`NewEnumerator0` 3 :`NewEnumerator1` 2 :`NewEnumerator2` 1)))))

(event `replay`
  (goto _label :!via `PlayFromStart`))

(event `self.Cube.OnComponentBeginOverlap`
  (params (OverlappedComponent :type "PrimitiveComponent Object Reference") (OtherActor :type "Actor Object Reference") (OtherComp :type "PrimitiveComponent Object Reference") (OtherBodyIndex :type Integer) (bFromSweep :type Boolean) (SweepResult :type "HitResult Structure (by ref)"))
  (bind _asbp_third_person_character (cast `/Game/ThirdPerson/Blueprints/BP_ThirdPersonCharacter` OtherActor))
  (bind _butin (`/Game/ThirdPerson/Blueprints/BP_ThirdPersonCharacter.Butin` _asbp_third_person_character))
  (if (< _butin 10)
    (`/Engine/EditorBlueprintResources/StandardMacros.IncrementInt` _butin
      (:`  `
        (`self.K2_DestroyActor` self)
        (`KismetSystemLibrary.PrintString` (`KismetStringLibrary.Conv_IntToString` _butin))))
    (else
      (`KismetSystemLibrary.PrintString` "full"))))

(fn `UserConstructionScript`
  (bind _cube (`self.Cube`))
  (bind _typecollectible (`self.TypeCollectible`))
  (`StaticMeshComponent.SetStaticMesh` _cube (select `int` _typecollectible :`0` "/Game/Fab/Bread_Low_Poly/bread_low_poly/StaticMeshes/bread_low_poly.bread_low_poly" :`1` "/Game/Fab/Red_Velvet/415bbf00_e769_4541_9110_d75982c1f609.415bbf00_e769_4541_9110_d75982c1f609" :`2` "/Game/Fab/CC0_-_Croissant/cc0_croissant/StaticMeshes/cc0_croissant.cc0_croissant" :!type "StaticMesh Object Reference"))
  (`SceneComponent.SetWorldScale3D` _cube (select `int` _typecollectible :`0` (8.0 8.0 8.0) :`1` (1.0 1.0 1.0) :`2` (8.0 8.0 8.0) :!type "Vector Structure")))